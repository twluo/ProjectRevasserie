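; Hex tile actor that highlights its surrounding area on a hex map when clicked.
; On click, it asks its owning hexTileMap for the tiles within range 2 of its X/Y coordinates and swaps each one's mesh material to a pulsing tech material.
; Nothing in this graph restores the original material.
; The construction script scales the tile horizontally by its Size variable.
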(event `self.ReceiveBeginPlay`)

(event `self.ReceiveActorBeginOverlap`
  (params (OtherActor :type "Actor Object Reference")))

(event `self.ReceiveTick`
  (params (DeltaSeconds :type "Float (single-precision)")))

(event `self.hexTile.OnClicked`
  (params (TouchedComponent :type "PrimitiveComponent Object Reference"))
  (bind _ashex_tile_map (cast `/Game/Blueprints/hexTileMap` (`self.GetOwner` self)))
  (bind _returnvalue (`board.getTilesInRange` _ashex_tile_map (`self.X`) (`self.Y`) 2))
  (for _array_element _returnvalue
    (if (`KismetSystemLibrary.IsValid` _array_element)
      (bind _ashex_tile_bp (cast `/Game/Blueprints/hexTileBP` _array_element))
      (`PrimitiveComponent.SetMaterial` (`/Game/Blueprints/hexTileBP.hexTile` _ashex_tile_bp) 0 "/Game/StarterContent/Materials/M_Tech_Hex_Tile_Pulse.M_Tech_Hex_Tile_Pulse"))))

(fn `UserConstructionScript`
  (bind _size (`self.Size`))
  (`self.SetActorScale3D` (`KismetMathLibrary.MakeVector` _size _size 1.0)))