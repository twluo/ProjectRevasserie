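; Hex board actor that spawns a grid of hexTileBP tiles, tracks characters on it and highlights movement ranges.
; Construction scales hex dimensions and sizes the CameraBounds box to the board.
; BeginPlay fills MapArray with tiles, gives each a dynamic material, then snaps CharacterList characters to their tiles.
; Selection stores the tiles in range and tints them by Cost through a material parameter, resetting them to white on deselect.
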(event `self.ReceiveBeginPlay`
  ;[1 1 1] Setting the board up
  (for _index (range (`self.NumOfTilesY`))
    (for _index_2 (range (`self.NumOfTilesX`))
      (bind (_x_pos _y_pos) (`self.Get Position` _index_2 _index))
      (bind _returnvalue (`|SpawnActorFromClass` "/Game/Blueprints/Map/hexTileBP.hexTileBP_C" (`KismetMathLibrary.MakeTransform` (+ (`KismetMathLibrary.MakeVector` _x_pos _y_pos) (`self.K2_GetActorLocation`))) false self (`self.TileSize`) _index_2 _index 1))
      (bind _returnvalue_2 (`KismetArrayLibrary.Array_Add` (`self.mapArray`) _returnvalue))
      (bind _hextile (`/Game/Blueprints/Map/hexTileBP.hexTile` _returnvalue))
      (bind _returnvalue_3 (`PrimitiveComponent.CreateDynamicMaterialInstance` _hextile 0 "/Game/Materials/M_Tech_Hex_Tile.M_Tech_Hex_Tile"))
      (`PrimitiveComponent.SetMaterial` _hextile 0 _returnvalue_3)
      (set `/Game/Blueprints/Map/hexTileBP.TileMaterial` _returnvalue_3 _returnvalue)))
  (`self.Spawn Characters`))

(fn `Deselect Tiles in Range`
  (for _array_element (`self.Selected Tiles`)
    (if (`KismetSystemLibrary.IsValid` _array_element)
      (bind _ashex_tile_bp (cast `/Game/Blueprints/Map/hexTileBP` _array_element))
      (`MaterialInstanceDynamic.SetVectorParameterValue` (`/Game/Blueprints/Map/hexTileBP.TileMaterial` _ashex_tile_bp) "Highlight Color" (struct :`R` 1.0 :`G` 1.0 :`B` 1.0 :`A` 1.0))
      (set `self.Selected Flag` false))))

(fn `Get Character`
  (params (X :type Integer) (Y :type Integer))
  (returns (Character :type "basicCharacter Object Reference"))
  (for _array_element (`self.Character List`)
    (if (and (== X (`basicCharacter.x` _array_element)) (== Y (`basicCharacter.y` _array_element)))
      (return _array_element)))
  (return _array_element))

(fn `Move Character`
  (params (X :type Integer) (Y :type Integer) (Character :type "basicCharacter Object Reference"))
  (`basicCharacter.setLocation` Character X Y)
  (bind _returnvalue (`self.getTile` X Y))
  (`/Engine/EditorBlueprintResources/StandardMacros.IsValid` _returnvalue
    (:`Is Valid`
      (`self.K2_SetActorLocation` Character (`self.K2_GetActorLocation` _returnvalue) false))))

(fn `Select Tiles in Range`
  (params (X :type Integer) (Y :type Integer) (Range :type Integer) (Character :type "basicCharacter Object Reference"))
  (if (!= Range 0)
    (set `self.Selected Character` Character)
    (bind _output_get (set `self.Selected X` X))
    (bind _output_get_2 (set `self.Selected Y` Y))
    (bind _returnvalue (`self.getTilesInRange` _output_get _output_get_2 Range))
    (bind _output_get_3 (set `self.Selected Tiles` _returnvalue))
    (for _array_element _output_get_3
      (if (`KismetSystemLibrary.IsValid` _array_element)
        (bind _ashex_tile_bp (cast `/Game/Blueprints/Map/hexTileBP` _array_element))
        (switch `int` (`boardTile.Cost` _array_element)
          (:`Default`
            (bind _tilematerial (`/Game/Blueprints/Map/hexTileBP.TileMaterial` _ashex_tile_bp))
            (`MaterialInstanceDynamic.SetVectorParameterValue` _tilematerial "Highlight Color" (struct :`G` 0.63 :`B` 0.624216 :`A` 1.0) :!label _label))
          (:`0`
            (`MaterialInstanceDynamic.SetVectorParameterValue` _tilematerial "Highlight Color" (struct :`R` 0.63 :`G` 0.101626 :`B` 0.549042 :`A` 1.0)))
          (:`1`
            (`MaterialInstanceDynamic.SetVectorParameterValue` _tilematerial "Highlight Color" (struct :`R` 0.090608 :`G` 0.63 :`A` 1.0)))
          (:`2`
            (`MaterialInstanceDynamic.SetVectorParameterValue` _tilematerial "Highlight Color" (struct :`R` 0.508567 :`G` 0.63 :`A` 1.0)))
          (:`3`
            (`MaterialInstanceDynamic.SetVectorParameterValue` _tilematerial "Highlight Color" (struct :`R` 0.63 :`A` 1.0)))
          (:`4`
            (`MaterialInstanceDynamic.SetVectorParameterValue` _tilematerial "Highlight Color" (struct :`R` 0.052053 :`B` 0.63 :`A` 1.0)))
          (:`5`
            (goto _label)))
        (set `self.Selected Flag` true)))))

(fn `Select/Deselect Tiles in Range`
  (params (X :type Integer) (Y :type Integer) (Range :type Integer) (SelectedCharacter :type "basicCharacter Object Reference"))
  (bind _returnvalue (== (`self.Selected Character`) SelectedCharacter))
  (if (`self.Selected Flag`)
    (if _returnvalue
      _
      (else
        _))
    (`self.Deselect Tiles in Range`)
    (if (not _returnvalue)
      (`self.Select Tiles in Range` X Y Range SelectedCharacter :!label _label))
    (else
      (goto _label))))

(fn `Spawn Characters`
  (for _array_element (`self.Character List`)
    (`self.Move Character` (`basicCharacter.x` _array_element) (`basicCharacter.y` _array_element) _array_element)))

(fn `UserConstructionScript`
  (bind _camerabounds (`self.CameraBounds`))
  (bind _returnvalue (`KismetMathLibrary.MakeVector` (* (+ (* (`self.NumOfTilesX`) (`self.Width`)) (/ (`self.Width`) 2.0)) 50.0) (* (+ (* (* (- (`self.NumOfTilesY`) 1) (/ (`self.Height`) 2.0)) 1.5) (`self.Height`)) -50.0) 1.0))
  (`self.Set up Variables`)
  (`SceneComponent.K2_SetRelativeLocation` _camerabounds _returnvalue false)
  (`SceneComponent.SetRelativeScale3D` _camerabounds _returnvalue)
  (`BoxComponent.SetBoxExtent` _camerabounds (1.0 1.0 1.0) true))