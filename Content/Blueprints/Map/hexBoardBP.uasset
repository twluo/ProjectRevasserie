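; Hex board actor that builds a grid of hex tiles on BeginPlay and places the listed characters on their starting tiles.
; Each tile gets a dynamic material instance, letting highlight events tint movement ranges blue, or red when occupied (nonzero cost) or too costly, and reset to white.
; The construction script scales tile dimensions by tile size and fits the CameraBounds box to the board.
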(event `self.ReceiveBeginPlay`
  ;[1 1 1] Setting the board up
  (for _index (range (`self.NumOfTilesY`))
    (for _index_2 (range (`self.NumOfTilesX`))
      (bind (_x_pos _y_pos) (`self.Get Position` _index_2 _index))
      (bind _returnvalue (`|SpawnActorFromClass` "/Game/Blueprints/Map/hexTileBP.hexTileBP_C" (`KismetMathLibrary.MakeTransform` (+ (`KismetMathLibrary.MakeVector` _x_pos _y_pos) (`self.K2_GetActorLocation`))) "Undefined" "OverrideRootScale" self (`self.TileSize`) _index_2 _index 1))
      (`KismetArrayLibrary.Array_Add` (`self.mapArray`) _returnvalue)
      (bind _hextile (`/Game/Blueprints/Map/hexTileBP.hexTile` _returnvalue))
      (bind _returnvalue_2 (`PrimitiveComponent.CreateDynamicMaterialInstance` _hextile 0 "/Game/Materials/M_Tech_Hex_Tile.M_Tech_Hex_Tile"))
      (`PrimitiveComponent.SetMaterial` _hextile 0 _returnvalue_2)
      (set `/Game/Blueprints/Map/hexTileBP.TileMaterial` _returnvalue_2 _returnvalue)))
  (`self.Spawn Characters`))

(event `self.highlightTiles`
  (params (tilesInRange :type "Array of boardTile Object Reference (by ref)") (movementCost :type Integer))
  (`self.Highlight Tiles BP` tilesInRange movementCost))

(event `self.unhighlightTiles`
  (params (tilesInRange :type "Array of boardTile Object Reference (by ref)"))
  (`self.Unhighlight Tiles BP` tilesInRange))

(fn `Highlight Tiles BP`
  (params (`Tiles in Range` :type "Array of boardTile Object Reference") (`Movement Cost` :type Integer))
  (for _array_element `Tiles in Range`
    (bind _ashex_tile_bp (cast `/Game/Blueprints/Map/hexTileBP` _array_element))
    (bind _returnvalue (`boardTile.isOccupied` _ashex_tile_bp))
    (bind _cost (`boardTile.Cost` _ashex_tile_bp))
    (if (or (and _returnvalue (!= 0 _cost)) (> _cost `Movement Cost`))
      (bind _tilematerial (`/Game/Blueprints/Map/hexTileBP.TileMaterial` _ashex_tile_bp))
      (`MaterialInstanceDynamic.SetVectorParameterValue` _tilematerial "Highlight Color" (struct :`R` 1.0 :`A` 1.0))
      (else
        (`MaterialInstanceDynamic.SetVectorParameterValue` _tilematerial "Highlight Color" (struct :`B` 1.0 :`A` 1.0))))))

(fn `Spawn Characters`
  (for _array_element (`self.Character List`)
    (bind _asbasic_character_bp (cast `/Game/Blueprints/Character/basicCharacterBP` _array_element))
    (bind _returnvalue (`self.getTile` (`/Game/Blueprints/Character/basicCharacterBP.X` _asbasic_character_bp) (`/Game/Blueprints/Character/basicCharacterBP.Y` _asbasic_character_bp)))
    (`basicCharacter.setLocation` _asbasic_character_bp _returnvalue)
    (`/Game/Blueprints/Character/basicCharacterBP.Move BP` _asbasic_character_bp _returnvalue)))

(fn `Unhighlight Tiles BP`
  (params (tilesInRange :type "Array of boardTile Object Reference"))
  (for _array_element tilesInRange
    (bind _ashex_tile_bp (cast `/Game/Blueprints/Map/hexTileBP` _array_element))
    (`MaterialInstanceDynamic.SetVectorParameterValue` (`/Game/Blueprints/Map/hexTileBP.TileMaterial` _ashex_tile_bp) "Highlight Color" (struct :`R` 1.0 :`G` 1.0 :`B` 1.0 :`A` 1.0))))

(fn `UserConstructionScript`
  (bind _camerabounds (`self.CameraBounds`))
  (bind _returnvalue (`KismetMathLibrary.MakeVector` (* (+ (* (`self.NumOfTilesX`) (`self.Width`)) (/ (`self.Width`) 2.0)) 50.0) (* (+ (* (* (- (`self.NumOfTilesY`) 1) (/ (`self.Height`) 2.0)) 1.5) (`self.Height`)) -50.0) 1.0))
  (`self.Set up Variables`)
  (`SceneComponent.K2_SetRelativeLocation` _camerabounds _returnvalue false false)
  (`SceneComponent.SetRelativeScale3D` _camerabounds _returnvalue)
  (`BoxComponent.SetBoxExtent` _camerabounds (1.0 1.0 1.0) true))