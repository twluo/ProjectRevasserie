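; Hex tile actor for a tile map, acting as a clickable destination for moving the selected character.
; On click, if it is among the owning hexTileMap's selected tiles, it moves the character to its X/Y and subtracts its Cost from MovementRange.
; It then reselects tiles within the remaining range, or only clears the selection when none is left.
; The construction script scales it horizontally by Size.
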(event `self.ReceiveBeginPlay`)

(event `self.ReceiveActorBeginOverlap`
  (params (OtherActor :type "Actor Object Reference")))

(event `self.ReceiveTick`
  (params (DeltaSeconds :type "Float (single-precision)")))

(event `self.ReceiveActorOnClicked`
  (bind _x (`self.X`))
  (bind _y (`self.Y`))
  (bind _ashex_tile_map (cast `/Game/Blueprints/Map/hexTileMap` (`self.GetOwner` self)))
  (if (and (`/Game/Blueprints/Map/hexTileMap.Selected Flag` _ashex_tile_map) (`KismetArrayLibrary.Array_Contains` (`/Game/Blueprints/Map/hexTileMap.Selected Tiles` _ashex_tile_map) self))
    (bind _selected_character (`/Game/Blueprints/Map/hexTileMap.Selected Character` _ashex_tile_map))
    (`/Game/Blueprints/Map/hexTileMap.Set CharacterLocation` _ashex_tile_map _x _y _selected_character)
    (bind _output_get (set `basicCharacter.movementRange` (- (`basicCharacter.movementRange` _selected_character) (`self.Cost`)) _selected_character))
    (if (> _output_get 0)
      (`/Game/Blueprints/Map/hexTileMap.Deselect Tiles in Range` _ashex_tile_map)
      (`/Game/Blueprints/Map/hexTileMap.Select Tiles in Range` _ashex_tile_map _x _y _output_get _selected_character)
      (else
        (`KismetSystemLibrary.PrintString` "Hello")
        (`/Game/Blueprints/Map/hexTileMap.Deselect Tiles in Range` _ashex_tile_map)))))

(fn `UserConstructionScript`
  (bind _size (`self.Size`))
  (`self.SetActorScale3D` (`KismetMathLibrary.MakeVector` _size _size 1.0)))