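; Square grid board actor that builds a map of SquareTileBP tiles when play begins.
; Nested loops spawn tiles offset from the board's root location by tile size, passing each its grid coordinates and a uniform movement cost.
; Each tile gets one of four random materials, which does not affect its cost.
; Tiles are stored row by row in MapTiles, with helpers for coordinate lookup and bounds checks.
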(event `self.ReceiveBeginPlay`
  ;[1 1 1] Setting the board up
  (for _index (range (`self.NumOfTilesX`))
    (for _index_2 (range (`self.NumOfTilesY`))
      (bind _returnvalue (`|SpawnActorFromClass` "/Game/Blueprints/Map/squareTileBP.squareTileBP_C" (`KismetMathLibrary.MakeTransform` (+ (`KismetMathLibrary.MakeVector` (* 100 (+ (/ (`self.TileSize`) 2.0) (* _index_2 (`self.TileSize`)))) (* -100 (+ (* _index (`self.TileSize`)) (/ (`self.TileSize`) 2.0)))) (`SceneComponent.K2_GetComponentLocation` (`self.DefaultSceneRoot`))) (struct) (1.0 1.0 1.0)) false self (`self.TileSize`) _index_2 _index 1))
      (`KismetArrayLibrary.Array_Add` (`self.MapTiles`) _returnvalue)
      ;;[1 1 1] Assigning Texture
      (switch `int` (`KismetMathLibrary.RandomInteger` 4)
        (:`0`
          (bind _tile (`/Game/Blueprints/Map/squareTileBP.Tile` _returnvalue))
          (`PrimitiveComponent.SetMaterial` _tile 0 "/Game/Materials/M_Brick_Clay_New.M_Brick_Clay_New"))
        (:`1`
          (`PrimitiveComponent.SetMaterial` _tile 0 "/Game/Materials/M_CobbleStone_Pebble.M_CobbleStone_Pebble"))
        (:`2`
          (`PrimitiveComponent.SetMaterial` _tile 0 "/Game/Materials/M_Concrete_Tiles.M_Concrete_Tiles"))
        (:`3`
          (`PrimitiveComponent.SetMaterial` _tile 0 "/Game/Materials/M_Water_Ocean.M_Water_Ocean"))))))

(fn `Get Tile`
  (params (X :type Integer) (Y :type Integer))
  (returns (`Map Tile` :type "/Game/Blueprints/Map/squareTileBP Object Reference"))
  (return (`KismetArrayLibrary.Array_Get` (`self.MapTiles`) (+ X (* Y (`self.NumOfTilesX`))))))

(fn `UserConstructionScript`)

(fn `Within Bounds`
  (params (X :type Integer) (Y :type Integer))
  (returns (`Within Bounds` :type Boolean))
  (return (and (< X (`self.NumOfTilesX`)) (>= X 0) (< Y (`self.NumOfTilesY`)) (>= Y 0))))