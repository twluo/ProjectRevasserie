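; Map generator actor that builds the game board as a grid of MapTile actors on BeginPlay.
; Nested loops over the X and Y tile counts spawn tiles scaled by TileSize, centered in their cells and offset from the actor's root location.
; Each tile is owned by the generator and tagged with its two grid indices.
; A random choice among four ground materials is present but disconnected, so it never runs.
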(event `self.ReceiveBeginPlay`
  (bind _tilesize (`self.TileSize`))
  ;[1 1 1] Setting the board up
  (for _index (range (`self.NumOfTilesX`))
    (for _index_2 (range (`self.NumOfTilesY`))
      (bind _returnvalue (`|SpawnActorFromClass` "/Game/Blueprints/mapTile.mapTile_C" (`KismetMathLibrary.MakeTransform` (+ (`KismetMathLibrary.MakeVector` (* 100 (+ (/ _tilesize 2.0) (* _index_2 (`self.TileSize`)))) (* 100 (+ (* _index (`self.TileSize`)) (/ (`self.TileSize`) 2.0)))) (`SceneComponent.K2_GetComponentLocation` (`self.DefaultSceneRoot`))) (struct) (`KismetMathLibrary.MakeVector` _tilesize _tilesize 1.0)) false self (`self.TileSize`)))
      (set `Actor.Tags` (`|MakeArray` (`KismetStringLibrary.Conv_StringToName` (`KismetStringLibrary.Conv_IntToString` _index_2)) (`KismetStringLibrary.Conv_StringToName` (`KismetStringLibrary.Conv_IntToString` _index))) _returnvalue))))

(fn `UserConstructionScript`)