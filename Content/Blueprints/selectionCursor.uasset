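; Selection cursor actor that marks a tile with a static mesh and keeps track of that tile's coordinates.
; The construction script scales the actor in X and Y by Size.
; SetLocation stores the tile indices and moves the mesh to the given world X/Y, just above zero height.
; The event graph is empty, and GetTileCoords has no wired logic.
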(event `self.ReceiveBeginPlay`)

(event `self.ReceiveActorBeginOverlap`
  (params (OtherActor :type "Actor Object Reference")))

(event `self.ReceiveTick`
  (params (DeltaSeconds :type "Float (single-precision)")))

(fn `SetLocation`
  (params (X :type "Float (double-precision)") (Y :type "Float (double-precision)") (`X Tile` :type Integer) (`Y Tile` :type Integer))
  (set `self.X Tile` `X Tile`)
  (set `self.Y Tile` `Y Tile`)
  (`SceneComponent.K2_SetWorldLocation` (`self.StaticMesh`) (`KismetMathLibrary.MakeVector` X Y 0.01) false))

(fn `UserConstructionScript`
  (bind _size (`self.Size`))
  (`self.SetActorScale3D` (`KismetMathLibrary.MakeVector` _size _size 1.0)))