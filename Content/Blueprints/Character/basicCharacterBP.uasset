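; Base character Blueprint for a tile-based movement game, clickable and able to move onto a given tile.
; Clicks are forwarded to the GameController, fetched from the gamemodeSettings game mode, through OnCharacterClicked.
; PostMove calls MoveBP, which snaps the actor to the tile's location without sweeping.
; The construction script initializes RemainingMoves from MovementRange, though nothing here decrements it.
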(event `self.ReceiveBeginPlay`)

(event `self.ReceiveActorOnClicked`
  (params (ButtonPressed :type "Key Structure" :default "AnyKey"))
  (bind _game_controller (`self.getGameController`))
  (`myGameController.onCharacterClicked` _game_controller self))

(event `self.postMove`
  (params (tile :type "boardTile Object Reference"))
  (`self.Move BP` tile))

(fn `getGameController`
  (returns (`Game Controller` :type "myGameController Object Reference"))
  (bind _asgamemode_settings (cast `/Game/Blueprints/gamemodeSettings` (`GameplayStatics.GetGameMode`))
    (:`then`
      _)
    (:`CastFailed`
      _))
  (return (`/Game/Blueprints/gamemodeSettings.Game Controller` _asgamemode_settings)))

(fn `Move BP`
  (params (Tile :type "boardTile Object Reference"))
  (`self.K2_SetActorLocation` (`self.K2_GetActorLocation` Tile)))

(fn `UserConstructionScript`
  (set `self.remainingMoves` (`self.movementRange`)))