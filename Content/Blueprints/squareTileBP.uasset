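; Square grid tile that, when clicked, prints and recolors with M_Door every tile within a movement range of five.
; Range search recurses through the four orthogonal neighbors via the owning squareTileMap, adding the current tile's MovementCost per step.
; An AddUnique accumulator removes duplicates, but tiles can be revisited since only the range limit stops recursion.
; The construction script scales the tile's X and Y by Size.
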(event `self.Tile.OnClicked`
  (params (TouchedComponent :type "PrimitiveComponent Object Reference"))
  (bind _tiles_in_range (`self.Get Tiles in Range` 5))
  (for _array_element _tiles_in_range
    (if (`KismetSystemLibrary.IsValid` _array_element)
      (`KismetSystemLibrary.PrintString` (`KismetStringLibrary.Concat_StrStr` "X = " (`KismetStringLibrary.Conv_IntToString` (`/Game/Blueprints/squareTileBP.X` _array_element)) " Y = " (`KismetStringLibrary.Conv_IntToString` (`/Game/Blueprints/squareTileBP.Y` _array_element))))
      (`PrimitiveComponent.SetMaterial` (`/Game/Blueprints/squareTileBP.Tile` _array_element) 0 "/Game/Materials/M_Door.M_Door"))))

(fn `Check Bottom`
  (params (Range :type Integer) (`Distance From Origin` :type Integer) (Accumulator :type "Array of /Game/Blueprints/squareTileBP Object Reference (by ref)") (Map :type "/Game/Blueprints/squareTileMap Object Reference"))
  (bind _x (`self.X`))
  (bind _returnvalue (+ (`self.Y`) -1))
  (bind _within_bounds (`/Game/Blueprints/squareTileMap.Within Bounds` Map _x _returnvalue))
  (if _within_bounds
    (bind _map_tile (`/Game/Blueprints/squareTileMap.Get Tile` Map _x _returnvalue))
    (`self.Get Tiles in Range (helper)` _map_tile Range (+ `Distance From Origin` (`self.Movement Cost`)) Accumulator)))

(fn `Check Left`
  (params (Range :type Integer) (`Distance From Origin` :type Integer) (Accumulator :type "Array of /Game/Blueprints/squareTileBP Object Reference (by ref)") (Map :type "/Game/Blueprints/squareTileMap Object Reference"))
  (bind _y (`self.Y`))
  (bind _returnvalue (+ (`self.X`) -1))
  (bind _within_bounds (`/Game/Blueprints/squareTileMap.Within Bounds` Map _returnvalue _y))
  (if _within_bounds
    (bind _map_tile (`/Game/Blueprints/squareTileMap.Get Tile` Map _returnvalue _y))
    (`self.Get Tiles in Range (helper)` _map_tile Range (+ `Distance From Origin` (`self.Movement Cost`)) Accumulator)))

(fn `Check Right`
  (params (Range :type Integer) (`Distance From Origin` :type Integer) (Accumulator :type "Array of /Game/Blueprints/squareTileBP Object Reference (by ref)") (Map :type "/Game/Blueprints/squareTileMap Object Reference"))
  (bind _y (`self.Y`))
  (bind _returnvalue (+ (`self.X`) 1))
  (bind _within_bounds (`/Game/Blueprints/squareTileMap.Within Bounds` Map _returnvalue _y))
  (if _within_bounds
    (bind _map_tile (`/Game/Blueprints/squareTileMap.Get Tile` Map _returnvalue _y))
    (`self.Get Tiles in Range (helper)` _map_tile Range (+ `Distance From Origin` (`self.Movement Cost`)) Accumulator)))

(fn `Check Top`
  (params (Range :type Integer) (`Distance From Origin` :type Integer) (Accumulator :type "Array of /Game/Blueprints/squareTileBP Object Reference (by ref)") (Map :type "/Game/Blueprints/squareTileMap Object Reference"))
  (bind _x (`self.X`))
  (bind _returnvalue (+ (`self.Y`) 1))
  (bind _within_bounds (`/Game/Blueprints/squareTileMap.Within Bounds` Map _x _returnvalue))
  (if _within_bounds
    (bind _map_tile (`/Game/Blueprints/squareTileMap.Get Tile` Map _x _returnvalue))
    (`self.Get Tiles in Range (helper)` _map_tile Range (+ `Distance From Origin` (`self.Movement Cost`)) Accumulator)))

(fn `Get Tiles in Range`
  (params (Range :type Integer))
  (returns (`Tiles in Range` :type "Array of /Game/Blueprints/squareTileBP Object Reference"))
  (bind _acuumulator (`self.Get Tiles in Range (helper)` Range 0 (`|MakeArray` null :!type "/Game/Blueprints/squareTileBP Object Reference")))
  (return _acuumulator))

(fn `Get Tiles in Range (helper)`
  (params (Range :type Integer) (`Distance from Origin` :type Integer) (Accumulator :type "Array of /Game/Blueprints/squareTileBP Object Reference"))
  (returns (Acuumulator :type "Array of /Game/Blueprints/squareTileBP Object Reference"))
  (if (>= Range `Distance from Origin`)
    (`KismetArrayLibrary.Array_AddUnique` Accumulator self)
    (bind _assquare_tile_map (cast `/Game/Blueprints/squareTileMap` (`self.GetOwner` self))
      (:`then`
        (`self.Check Top` Range `Distance from Origin` Accumulator _assquare_tile_map)
        (`self.Check Bottom` Range `Distance from Origin` Accumulator _assquare_tile_map)
        (`self.Check Left` Range `Distance from Origin` Accumulator _assquare_tile_map)
        (`self.Check Right` Range `Distance from Origin` Accumulator _assquare_tile_map))
      (:`CastFailed`
        _)))
  (return Accumulator))

(fn `UserConstructionScript`
  (bind _size (`self.Size`))
  ;[1 1 1] Set the size
  (`self.SetActorScale3D` (`KismetMathLibrary.MakeVector` _size _size 1.0)))