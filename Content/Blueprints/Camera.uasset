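; Free-moving camera actor that pans with input axes or screen-edge mouse position and zooms along its view direction.
; Forward/Backward, Left/Right and Zoom graphs compute offsets scaled by CameraSpeed, with mouse wheel presses giving brief zoom pulses.
; The Left/Right axis event sums all three offsets and moves the actor only if a forward trace from the proposed position hits, constraining where the camera can go.
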(event `InputAxis|Left/Right`
  (params (AxisValue :type "Float (single-precision)"))
  (bind _returnvalue (`SceneComponent.GetForwardVector` (`self.Camera`)))
  (bind _returnvalue_2 (+ (`self.Left/Right`) (`self.K2_GetActorLocation`) (`self.Forward/Backward`) (`self.Zoom In/Out`)))
  (bind (_outhit _returnvalue_3) (`KismetSystemLibrary.LineTraceSingle` (+ _returnvalue_2 (* _returnvalue 100.0)) (+ _returnvalue_2 (* _returnvalue 10000.0)) "TraceTypeQuery3"))
  (if _returnvalue_3
    (`self.K2_SetActorRelativeLocation` _returnvalue_2)))

(event `Key|MouseScrollUp`
  (:`Pressed`
    (set `self.Mouse Zoom In/Out` 1.0)
    (`KismetSystemLibrary.Delay` 0.2 :!label _label)
    (set `self.Mouse Zoom In/Out` 0.0)))

(event `Key|MouseScrollDown`
  (:`Pressed`
    (set `self.Mouse Zoom In/Out` -1.0)
    (goto _label)))

(fn `UserConstructionScript`
  (`KismetSystemLibrary.PrintString` (`KismetStringLibrary.Conv_VectorToString` (`self.K2_GetActorLocation`))))