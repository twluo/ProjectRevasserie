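; Hex grid map actor that spawns a board of HexTileBP tiles at BeginPlay.
; It scales tile width and height by TileSize, then loops over both axes, spawning each tile with its coordinates and storing it in MapArray.
; Get Position supplies tile locations, with math for staggering odd rows by half a width.
; Each tile gets one of four random surface materials and the same movement cost.
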(event `self.ReceiveBeginPlay`
  ;[1 1 1] Setting the board up
  (`self.Set up Variables`)
  (for _index (range (`self.NumOfTilesX`))
    (for _index_2 (range (`self.NumOfTilesY`))
      (bind (_x_pos _y_pos) (`self.Get Position` _index_2 _index))
      (bind _returnvalue (`|SpawnActorFromClass` "/Game/Blueprints/hexTileBP.hexTileBP_C" (`KismetMathLibrary.MakeTransform` (`KismetMathLibrary.MakeVector` _x_pos _y_pos)) false self (`self.TileSize`) _index_2 _index 1))
      (`KismetArrayLibrary.Array_Add` (`self.mapArray`) _returnvalue)
      (switch `int` (`KismetMathLibrary.RandomInteger` 4)
        (:`0`
          (bind _hextile (`/Game/Blueprints/hexTileBP.hexTile` _returnvalue))
          (`PrimitiveComponent.SetMaterial` _hextile 0 "/Game/Materials/M_Brick_Clay_New.M_Brick_Clay_New"))
        (:`1`
          (`PrimitiveComponent.SetMaterial` _hextile 0 "/Game/Materials/M_CobbleStone_Pebble.M_CobbleStone_Pebble"))
        (:`2`
          (`PrimitiveComponent.SetMaterial` _hextile 0 "/Game/Materials/M_Concrete_Tiles.M_Concrete_Tiles"))
        (:`3`
          (`PrimitiveComponent.SetMaterial` _hextile 0 "/Game/Materials/M_Water_Ocean.M_Water_Ocean"))))))

(fn `UserConstructionScript`)